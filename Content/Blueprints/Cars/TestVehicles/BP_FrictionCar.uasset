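; Test vehicle Blueprint for a physics car with a body and wheels, driven by gamepad input.
; The triggers set a forward or reverse ForwardForce, with delayed checks arbitrating when both are held, and the MoveRight axis snaps TurningTorque to left, right or zero.
; Nothing here applies those values: Tick is empty, and the body-force, wheel-torque and angular-velocity experiments are disconnected and never run.
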(event `Key|Gamepad_RightTrigger`
  (params (Key :type "Key Structure"))
  (:`Pressed`
    (set `self.RightTriggerDown` true)
    (set `self.ForwardForce` (`self.DefaultForce`) :!label _label)
    (`KismetSystemLibrary.Delay` 0.1)
    (if (`self.LeftTriggerDown`)
      (set `self.RightTriggerDown` false)
      (set `self.ForwardForce` (* (`self.DefaultForce`) -1.0) :!label _label_2)
      (`KismetSystemLibrary.Delay` 0.1)
      (if (`self.RightTriggerDown`)
        (set `self.LeftTriggerDown` false)
        (goto _label))))
  (:`Released`
    (set `self.RightTriggerDown` false)
    (if (not (`self.LeftTriggerDown`))
      (set `self.ForwardForce` 1.0 :!label _label_3))))

(event `Key|Gamepad_LeftTrigger`
  (params (Key :type "Key Structure"))
  (:`Pressed`
    (set `self.LeftTriggerDown` true)
    (goto _label_2))
  (:`Released`
    (set `self.LeftTriggerDown` false)
    (if (not (`self.RightTriggerDown`))
      (goto _label_3))))

(event `InputAxis|MoveRight`
  (params (AxisValue :type "Float (single-precision)"))
  (bind _defaulttorque (`self.DefaultTorque`))
  (if (>= AxisValue 0.5)
    (set `self.TurningTorque` _defaulttorque)
    (elif (<= AxisValue -0.5)
      (set `self.TurningTorque` (* _defaulttorque -1.0))
      (else
        (set `self.TurningTorque` 0.0)))))

(event `self.ReceiveTick`
  (params (DeltaSeconds :type "Float (single-precision)")))

(fn `UserConstructionScript`)