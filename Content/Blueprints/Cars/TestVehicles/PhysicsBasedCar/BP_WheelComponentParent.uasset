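; Parent wheel component for the physics-based BP_ForceCar, providing raycast suspension and steering side force.
; On BeginPlay it maps the car's normalized tuning values to ride height, spring, damping and friction.
; Each tick a downward trace positions the selected wheel mesh and applies a spring-damper force at the component's location.
; When yawed, it also pushes the car body sideways along its right vector, weakening with speed to a floor.
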(event `self.ReceiveBeginPlay`
  (bind _asbp_force_car (cast `/Game/Blueprints/Cars/TestVehicles/PhysicsBasedCar/BP_ForceCar` (`self.GetOwner`)))
  (bind _output_get (set `self.BP_CarParent` _asbp_force_car))
  (set `self.DistanceToGround` (`KismetMathLibrary.Lerp` 50.0 250.0 (`/Game/Blueprints/Cars/TestVehicles/PhysicsBasedCar/BP_ForceCar.DistanceToGround` _output_get)))
  (set `self.SpringCoefficient` (`KismetMathLibrary.Lerp` 200.0 1000.0 (`/Game/Blueprints/Cars/TestVehicles/PhysicsBasedCar/BP_ForceCar.SuspensionStifness` _output_get)))
  (set `self.DampingCoefficient` (`KismetMathLibrary.Lerp` 20.0 180.0 (`/Game/Blueprints/Cars/TestVehicles/PhysicsBasedCar/BP_ForceCar.SuspensionBouciness` _output_get)))
  (set `self.FrontWeelsFriction` (`KismetMathLibrary.Lerp` 10000.0 150000.0 (`/Game/Blueprints/Cars/TestVehicles/PhysicsBasedCar/BP_ForceCar.HighSpeedDriftControl` _output_get))))

(event `self.ReceiveTick`
  (params (DeltaSeconds :type "Float (single-precision)"))
  (bind _returnvalue (`self.K2_GetComponentLocation`))
  (bind _bp_carparent (`self.BP_CarParent`))
  (bind (_relativerotation_roll _relativerotation_pitch _relativerotation_yaw) (`KismetMathLibrary.BreakRotator` (`self.RelativeRotation`)))
  (bind _returnvalue_2 (* (`self.GetRightVector`) (* (`KismetMathLibrary.FClamp` (/ (- 2000.0 (`KismetMathLibrary.VSize` (`Actor.GetVelocity` (`self.BP_CarParent`)))) 2000.0) 0.7) (`self.FrontWeelsFriction`))))
  (`/Engine/EditorBlueprintResources/StandardMacros.IsValid` (`self.BP_CarParent`)
    (:`Is Valid`
      (bind (_outhit _returnvalue_3) (`KismetSystemLibrary.LineTraceSingle` :`Start` _returnvalue :`End` (- _returnvalue (* (`self.GetUpVector`) (`self.DistanceToGround`))) :`TraceChannel` "TraceTypeQuery1" :`DrawDebugType` "ForOneFrame"))
      (if _returnvalue_3
        (bind (_bblockinghit _binitialoverlap _time _distance _location) (`GameplayStatics.BreakHitResult` _outhit))
        (`self.K2_SetWorldLocation` (select `int` (`self.WheelLocation(FL,FR, BL, BR)`) :`0` (`/Game/Blueprints/Cars/TestVehicles/PhysicsBasedCar/BP_ForceCar.FLWheel` _bp_carparent) :`1` (`/Game/Blueprints/Cars/TestVehicles/PhysicsBasedCar/BP_ForceCar.FRWheel` _bp_carparent) :`2` (`/Game/Blueprints/Cars/TestVehicles/PhysicsBasedCar/BP_ForceCar.BLWheel` _bp_carparent) :`3` (`/Game/Blueprints/Cars/TestVehicles/PhysicsBasedCar/BP_ForceCar.BRWheel` _bp_carparent)) (+ _location (0.0 0.0 40.0)) false false)
        (bind _output_get (set `self.HoverDelta` (- (`self.DistanceToGround`) _distance)))
        (`PrimitiveComponent.AddForceAtLocation` (cast `PrimitiveComponent` (`Actor.RootComponent` (`self.BP_CarParent`)) :!pure true) (* (`self.GetUpVector`) (+ (* (/ (- _output_get (`self.PreviousHoverDelta`)) (/ (`GameplayStatics.GetWorldDeltaSeconds`) 0.8)) (`self.DampingCoefficient`)) (* _output_get (`self.SpringCoefficient`)))) (`self.K2_GetComponentLocation`) "None")
        (set `self.PreviousHoverDelta` (`self.HoverDelta`))
        (`PrimitiveComponent.AddForce` (cast `PrimitiveComponent` (`Actor.RootComponent` (`self.BP_CarParent`)) :!pure true) (select `bool` (`KismetMathLibrary.NearlyEqual_FloatFloat` _relativerotation_yaw 0.0 1.0) :`false` (select `bool` (> _relativerotation_yaw 0.0) :`false` (* _returnvalue_2 -1.0) :`true` _returnvalue_2)) "None" false)))))