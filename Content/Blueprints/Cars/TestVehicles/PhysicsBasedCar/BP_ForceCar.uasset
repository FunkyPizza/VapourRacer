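; Physics-driven test car pawn that turns by applying torque to its CenterOfMass body each tick.
; Gamepad triggers set a forward or reverse force value, but the AddForce call that would use it is disconnected.
; The MoveRight axis selects fixed left, right or zero torque and snaps two steering wheel components to match.
; Tick also points a Velocity component along the body's linear velocity.
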(event `self.ReceiveBeginPlay`
  (set `self.DefaultForce` (`KismetMathLibrary.Lerp` 150000.0 300000.0 (`self.GroundVelocity`)))
  (set `self.DefaultTorque` (`KismetMathLibrary.Lerp` 25000000.0 100000000.0 (`self.TorqueForce`))))

(event `Key|Gamepad_RightTrigger`
  (params (Key :type "Key Structure"))
  (:`Pressed`
    (set `self.RightTriggerDown` true)
    (set `self.ForwardForce` (`self.DefaultForce`) :!label _label)
    (`KismetSystemLibrary.Delay` 0.1)
    (if (`self.LeftTriggerDown`)
      (set `self.RightTriggerDown` false)
      (set `self.ForwardForce` (* (`self.DefaultForce`) -1.0) :!label _label_2)
      (`KismetSystemLibrary.Delay` 0.1)
      (if (`self.RightTriggerDown`)
        (set `self.LeftTriggerDown` false)
        (goto _label))))
  (:`Released`
    (set `self.RightTriggerDown` false)
    (if (not (`self.LeftTriggerDown`))
      (set `self.ForwardForce` 1.0 :!label _label_3))))

(event `Key|Gamepad_LeftTrigger`
  (params (Key :type "Key Structure"))
  (:`Pressed`
    (set `self.LeftTriggerDown` true)
    (goto _label_2))
  (:`Released`
    (set `self.LeftTriggerDown` false)
    (if (not (`self.RightTriggerDown`))
      (goto _label_3))))

(event `InputAxis|MoveRight`
  (params (AxisValue :type "Float (single-precision)"))
  (bind _defaulttorque (`self.DefaultTorque`))
  (if (>= AxisValue 0.5)
    (set `self.TurningTorque` _defaulttorque)
    (`SceneComponent.K2_SetRelativeRotation` (`self.BP_SteeringWheelComponentParent`) (struct :`Yaw` 30.0) false false)
    (`SceneComponent.K2_SetRelativeRotation` (`self.BP_SteeringWheelComponentParent1`) (struct :`Yaw` 30.0) false false)
    (elif (<= AxisValue -0.5)
      (set `self.TurningTorque` (* _defaulttorque -1.0))
      (`SceneComponent.K2_SetRelativeRotation` (`self.BP_SteeringWheelComponentParent`) (struct :`Yaw` -30.0) false false)
      (`SceneComponent.K2_SetRelativeRotation` (`self.BP_SteeringWheelComponentParent1`) (struct :`Yaw` -30.0) false false)
      (else
        (set `self.TurningTorque` 0.0)
        (`SceneComponent.K2_SetRelativeRotation` :`self` (`self.BP_SteeringWheelComponentParent`))
        (`SceneComponent.K2_SetRelativeRotation` :`self` (`self.BP_SteeringWheelComponentParent1`))))))

(event `self.ReceiveTick`
  (params (DeltaSeconds :type "Float (single-precision)"))
  (`PrimitiveComponent.AddTorqueInDegrees` (`self.CenterOfMass`) (* (`self.GetActorUpVector`) (`self.TurningTorque`)) "None" false)
  (bind _returnvalue (`PrimitiveComponent.GetPhysicsLinearVelocity` (`self.CenterOfMass`) "None"))
  (`SceneComponent.K2_SetWorldRotation` (`self.Velocity`) (`KismetMathLibrary.Conv_VectorToRotator` _returnvalue) false false))

(fn `UserConstructionScript`)