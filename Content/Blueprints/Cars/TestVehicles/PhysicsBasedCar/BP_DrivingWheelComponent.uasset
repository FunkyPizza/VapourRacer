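; Driving wheel component for a physics-based test car that propels the vehicle while the wheel is near the ground.
; Each tick it line-traces along its down vector by DistanceToGround on the Visibility channel, drawing a one-frame debug line.
; On a hit, it adds the car's ForwardForce to the CenterOfMass component, directed along the steering wheel component's forward vector.
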(event `self.ReceiveBeginPlay`
  (`parent.ReceiveBeginPlay`))

(event `self.ReceiveTick`
  (params (DeltaSeconds :type "Float (single-precision)"))
  (bind _returnvalue (`self.K2_GetComponentLocation`))
  (`parent.ReceiveTick` DeltaSeconds)
  (bind (_outhit _returnvalue_2) (`KismetSystemLibrary.LineTraceSingle` :`Start` _returnvalue :`End` (- _returnvalue (* (`self.GetUpVector`) (`self.DistanceToGround`))) :`TraceChannel` "TraceTypeQuery1" :`DrawDebugType` "ForOneFrame"))
  (if _returnvalue_2
    (`PrimitiveComponent.AddForce` (`/Game/Blueprints/Cars/TestVehicles/PhysicsBasedCar/BP_ForceCar.CenterOfMass` (`self.BP_CarParent`)) (* (`self.GetForwardVector` (`/Game/Blueprints/Cars/TestVehicles/PhysicsBasedCar/BP_ForceCar.BP_SteeringWheelComponentParent` (`self.BP_CarParent`))) (`/Game/Blueprints/Cars/TestVehicles/PhysicsBasedCar/BP_ForceCar.ForwardForce` (`self.BP_CarParent`))) "None" false)))