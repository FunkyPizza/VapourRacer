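; Arcade hover-car actor with gamepad driving, named as the blue main menu show car.
; Tick moves it along its forward vector by Speed, applies pedal-release friction and runs box-trace height correction with fallback gravity.
; Timelines ramp acceleration, braking and reverse, while drifting uses a short Delay loop for side slide and yaw inertia.
; Mesh-rotation timelines animate random idle bobbing, drift lean and impact tilts chosen from the hit normal.
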(event `self.ReceiveBeginPlay`
  ;[0.2344 0 0] Begin Play, Tick & Live Functions
  (`self.CarIdleAnimation`)
  (set `self.TempAnimOriginalRotation` (`SceneComponent.RelativeRotation` (`self.CarMesh`))))

(event `self.ReceiveTick`
  (params (DeltaSeconds :type "Float (single-precision)"))
  ;[0.2344 0 0] Begin Play, Tick & Live Functions
  ;;[1 1 1] Apply vehicle speed
  (`self.K2_AddActorWorldOffset` (* (`self.GetActorForwardVector`) (`self.Speed`)) true)
  ;;[1 1 1] Apply tyre friciton when both pedals are release & when reversing
  (if (or (`self.isBreaking`) (`self.isAccelerating`))
    _
    (elif (< (`self.Speed`) 0.0)
      (set `self.Speed` (`KismetMathLibrary.FClamp` (+ (`self.Speed`) (`self.SpeedlossWhenPedalsReleased`)) (`self.MaxReverseSpeed`) 0.0))
      (else
        (set `self.Speed` (`KismetMathLibrary.FClamp` (- (`self.Speed`) (`self.SpeedlossWhenPedalsReleased`)) 0.0 (`self.MaxSpeed`))))))
  ;;[1 1 1] Gravity & Anti-gravity
  (`self.ApplyGravity`))

(event `StartMovements`
  ;[0.2344 0 0] Begin Play, Tick & Live Functions
  (set `self.canMove` true)
  (`WidgetBlueprintLibrary.SetInputMode_GameOnly` (cast `/Game/Blueprints/GameMode/PC_PlayerCar` (`self.GetController`) :!pure true)))

(event `Impact`
  ;[0.2344 0 0] Begin Play, Tick & Live Functions
  ;;[1 1 1] Collision with other objects
  (set `self.Speed` 0.0)
  (`self.ReleasePedals`))

(event `self.CarCollision.OnComponentHit`
  (params (HitComponent :type "PrimitiveComponent Object Reference") (OtherActor :type "Actor Object Reference") (OtherComp :type "PrimitiveComponent Object Reference") (NormalImpulse :type "Vector Structure") (Hit :type "HitResult Structure (by ref)"))
  ;[0.2344 0 0] Begin Play, Tick & Live Functions
  ;;[1 1 1] Collision with other objects
  (`self.Impact Animation` Hit_Normal)
  (`self.Impact`))

(event `StopMovements`
  ;[0.2344 0 0] Begin Play, Tick & Live Functions
  (set `self.canMove` false)
  (`self.Break`))

(event `Key|Gamepad_RightTrigger`
  (params (Key :type "Key Structure"))
  ;[0 0 0] Throttle, Break & Reverse Input
  (:`Pressed`
    (if (`self.canMove`)
      ;;[1 1 1] If player is drifting, don't accelerate
      (if (not (`self.isDrifting`))
        (`self.GoForward`))
      (set `self.isAccelerating` true)))
  (:`Released`
    (`self.ReleasePedals`)
    (set `self.isAccelerating` false)))

(event `InputAxis|MoveRight`
  (params (AxisValue :type "Float (single-precision)"))
  (bind _torquerate (`self.TorqueRate`))
  (bind _torquerate_2 (`self.TorqueRate`))
  ;[0 0 0] Torque Input
  (if (`self.canMove`)
    (if (>= AxisValue 0.5)
      ;;[1 1 1] Turning Right - Depending on drifting status & on current speed
      (`self.K2_AddActorWorldRotation` (`KismetMathLibrary.MakeRotator` 0.0 0.0 (* (select `bool` (`self.isDrifting`) :`false` _torquerate :`true` (/ _torquerate 3.0)) (`KismetMathLibrary.FClamp` (- 1.0 (/ (`self.Speed`) (`self.MaxSpeed`))) (`self.MinTorqueAtMaxSpeed(0 to 1)`)))))
      (else
        ;;[1 1 1] Turning Left - Depending on drifting status & on current speed
        (if (<= AxisValue -0.5)
          (`self.K2_AddActorWorldRotation` (`KismetMathLibrary.MakeRotator` 0.0 0.0 (* (select `bool` (`self.isDrifting`) :`false` (* _torquerate_2 -1.0) :`true` (/ _torquerate_2 -3.0)) (`KismetMathLibrary.FClamp` (- 1.0 (/ (`self.Speed`) (`self.MaxSpeed`))) (`self.MinTorqueAtMaxSpeed(0 to 1)`))))))))))

(event `InputReverse`
  ;[0 0 0] Throttle, Break & Reverse Input
  ;;[1 1 1] Select to break or reverse depending on car speed
  (`self.ReleasePedals` :!label _label)
  (`self.Reverse`)
  (set `self.isReversing` true)
  ;;[1 1 1] Rotate camera when reversing
  (`SceneComponent.K2_SetRelativeRotation` (`self.CameraSpring`) (struct :`Pitch` -10.0 :`Yaw` 180.0) false false))

(event `Key|Gamepad_LeftTrigger`
  (params (Key :type "Key Structure"))
  ;[0 0 0] Throttle, Break & Reverse Input
  (:`Pressed`
    (if (`self.canMove`)
      ;;[1 1 1] Select to break or reverse depending on car speed
      (if (<= (`self.Speed`) 0.0)
        (goto _label)
        (else
          (`KismetSystemLibrary.Delay` 0.2)
          (`self.Break`)
          (set `self.isBreaking` true)))))
  (:`Released`
    (set `self.isBreaking` false)
    (set `self.isReversing` false)
    (`self.ReleasePedals`)
    ;;[1 1 1] Make sure camera is facing forward
    (`SceneComponent.K2_SetRelativeRotation` (`self.CameraSpring`) (struct :`Pitch` -10.0) false false)
    ;;[1 1 1] Check if the player wants to accelerate
    (if (`self.isAccelerating`)
      (`self.GoForward`))))

(event `GoForward`
  ;[0 0 0] Throttle, Break, Reverse & Release Pedals
  ;;[1 1 1] Stop breaking & accelerate
  (`|ExecutionSequence`
    (:`then_0`
      ;;[1 1 1] Apply Break & Throttle
      (bind _output_get (set `self.TempForwardSpeed` (`self.Speed`)))
      (bind (_direction _newtrack_0) (`Timeline|AccelerationLerp` :`NewTime` (* (/ _output_get (`self.MaxSpeed`)) 5.0) :!via `PlayFromStart` :!label _label_2)
        (:`Update`
          (set `self.Speed` (`KismetMathLibrary.Lerp` (`self.TempForwardSpeed`) (`self.MaxSpeed`) _newtrack_0)))))
    (:`then_1`
      (bind (_direction_2 _newtrack_0_2) (`Timeline|BreakingLerp` :`NewTime` (* (/ (stale `Break` _output_get) (`self.MaxSpeed`)) 2.0) :!via `Stop` :!label _label_3)
        (:`Update`
          (set `self.Speed` (`KismetMathLibrary.Lerp` 0.0 (`self.TempForwardSpeed`) _newtrack_0_2)))
        (:`Finished`
          (if (`self.isBreaking`)
            (`self.InputReverse`)))))))

(event `Reverse`
  ;[0 0 0] Throttle, Break, Reverse & Release Pedals
  ;;[1 1 1] Apply reverse
  (bind _output_get (set `self.TempForwardSpeed` (`self.Speed`)))
  (bind (_direction _newtrack_0) (`Timeline|ReverseLerp` :`NewTime` (* (/ _output_get (`self.MaxReverseSpeed`)) 5.0) :!via `PlayFromStart` :!label _label_4)
    (:`Update`
      (set `self.Speed` (`KismetMathLibrary.Lerp` (`self.MaxReverseSpeed`) (`self.TempForwardSpeed`) _newtrack_0)))))

(event `ReleasePedals`
  ;[0 0 0] Throttle, Break, Reverse & Release Pedals
  ;;[1 1 1] Stop breaking and accelerating
  (`|ExecutionSequence`
    (:`then_0`
      (goto _label_2 :!via `Stop`))
    (:`then_1`
      (goto _label_3 :!via `Stop`))
    (:`then_2`
      (goto _label_4 :!via `Stop`))))

(event `Break`
  ;[0 0 0] Throttle, Break, Reverse & Release Pedals
  ;;[1 1 1] Stop accelerating & break
  (`|ExecutionSequence`
    (:`then_0`
      (goto _label_2 :!via `Stop`))
    (:`then_1`
      ;;[1 1 1] Apply Break & Throttle
      (bind _output_get (set `self.TempForwardSpeed` (`self.Speed`)))
      (goto _label_3 :!via `PlayFromStart`))))

(event `Key|Gamepad_RightShoulder`
  (params (Key :type "Key Structure"))
  (bind _carmesh (`self.CarMesh`))
  (bind _carmesh_2 (`self.CarMesh`))
  (bind _returnvalue (`KismetMathLibrary.Lerp` (`self.InertiaRotationAtEndOfDrift`) (`self.InertiaRotationAtStartOfDrift`) (/ (`self.Speed`) (`self.MaxSpeed`))))
  ;[0 0 0] Drifting Input & Movements
  (:`Pressed`
    (if (>= (`self.Speed`) (`self.MinimumSpeedToDrift`)) :!label _label_5
      (`self.ReleasePedals`)
      (set `self.isDrifting` true)
      (bind _output_get (set `self.isDriftingToTheRight` (< (`self.GetInputAxisValue`) 0.0)))
      (if _output_get :!label _label_6
        ;;[1 1 1] Forward velocity to drift speed convertion
        (bind _output_get_2 (set `self.TempLerpDrift` (`KismetMathLibrary.FClamp` (+ (`self.TempLerpDrift`) 0.015))))
        (bind _returnvalue_2 (* _output_get_2 (`self.Speed`) (`self.DriftSpeed`) -1.0))
        (bind _output_get_3 (set `self.TempDriftSideVelocity` (* (+ (`SceneComponent.GetRightVector` _carmesh_2) (* (`SceneComponent.GetForwardVector` _carmesh_2) 0.25)) (`KismetMathLibrary.MakeVector` _returnvalue_2 _returnvalue_2))))
        (`self.K2_AddActorWorldOffset` _output_get_3 true)
        ;;[1 1 1] Drift Loss Speed
        (set `self.Speed` (`KismetMathLibrary.FClamp` (- (`self.Speed`) (`self.DriftSpeedloss`)) 0.0 (`self.MaxSpeed`)))
        ;;[1 1 1] Drift Inertia
        (`self.K2_AddActorWorldRotation` (`KismetMathLibrary.MakeRotator` 0.0 0.0 (* _returnvalue -1.0)) true)
        ;;[1 1 1] Check if still drifting for next frame
        (`KismetSystemLibrary.Delay` 0.001)
        (if (`self.isDrifting`)
          (`self.DriftAnimation` :!label _label_7)
          (goto _label_6))
        (else
          (bind _output_get_4 (set `self.TempLerpDrift` (`KismetMathLibrary.FClamp` (+ (`self.TempLerpDrift`) 0.015))))
          (bind _returnvalue_3 (* _output_get_4 (`self.Speed`) (`self.DriftSpeed`)))
          (bind _output_get_5 (set `self.TempDriftSideVelocity` (* (+ (`SceneComponent.GetRightVector` _carmesh) (* (`SceneComponent.GetForwardVector` _carmesh) 0.25)) (`KismetMathLibrary.MakeVector` _returnvalue_3 _returnvalue_3))))
          (`self.K2_AddActorWorldOffset` _output_get_5 true)
          (set `self.Speed` (`KismetMathLibrary.FClamp` (- (`self.Speed`) (`self.DriftSpeedloss`)) 0.0 (`self.MaxSpeed`)))
          (`self.K2_AddActorWorldRotation` (`KismetMathLibrary.MakeRotator` 0.0 0.0 _returnvalue) true)
          (`KismetSystemLibrary.Delay` 0.001)
          (if (`self.isDrifting`)
            (goto _label_7))))))
  (:`Released`
    ;;[1 1 1] Check if still accelerating when done drifting
    (if (`self.isAccelerating`) :!label _label_8
      (`self.GoForward`))
    ;;[1 1 1] Reset Drift Variables
    (if (`self.isDrifting`)
      (set `self.TempLerpDrift` 0.0)
      (set `self.isDrifting` false)
      (`self.EndDriftAnimation`)
      ;;[1 1 1] Gradually reduce drift side velocity
      (bind (_direction _newtrack_0) (`Timeline|EndDriftVelocityLerp` :!via `PlayFromStart`)
        (:`Update`
          (`self.K2_AddActorWorldOffset` (`KismetMathLibrary.VLerp` (`self.TempDriftSideVelocity`) (0.0 0.0 0.0) _newtrack_0) true))))))

(event `Key|Gamepad_FaceButton_Bottom`
  (params (Key :type "Key Structure"))
  ;[0 0 0] Drifting Input & Movements
  (:`Pressed`
    (goto _label_5))
  (:`Released`
    (goto _label_8)))

(event `StopIdleAnimTimeline`
  (bind _returnvalue (`KismetMathLibrary.RandomFloatInRange` -5.0 5.0))
  (bind _returnvalue_2 (`KismetMathLibrary.RandomFloatInRange` -2.0 2.0))
  (bind _relativerotation (`SceneComponent.RelativeRotation` (`self.CarMesh`)))
  (bind _yaw (.yaw _relativerotation))
  ;[0.4323 0.1755 0] Idle Animation
  (set `self.isIdle` false)
  (bind (_direction _lerpvalue2s) (`Timeline|IdleAnimationLerp` :!via `Stop` :!label _label_9)
    (:`Update`
      ;;[1 1 1] Bobbing rotation
      (`SceneComponent.K2_SetRelativeRotation` (`self.CarMesh`) (`KismetMathLibrary.RLerp` (`self.TempAnimRotaA`) (`self.TempAnimRotaB`) _lerpvalue2s true) false false))
    (:`Finished`
      (`/Engine/EditorBlueprintResources/StandardMacros.FlipFlop` :!label _label_10
        (:`A`
          ;;[1 1 1] Set random bobbing rotation
          (set `self.TempAnimRotaA` _relativerotation)
          (set `self.TempAnimRotaB` (`KismetMathLibrary.MakeRotator` _returnvalue _returnvalue_2 _yaw))
          (goto _label_9 :!via `PlayFromStart`))
        (:`B`
          (set `self.TempAnimRotaA` (`KismetMathLibrary.MakeRotator` _returnvalue _returnvalue_2 _yaw))
          (goto _label_9 :!via `ReverseFromEnd`))))))

(event `CarIdleAnimation`
  ;[0.4323 0.1755 0] Idle Animation
  (set `self.isIdle` true)
  (set `self.TempCarSpringLocation` (`SceneComponent.RelativeLocation` (`self.CarMesh`)))
  (goto _label_10))

(event `DriftAnimation`
  (bind (_tempanimoriginalrotation_roll _tempanimoriginalrotation_pitch _tempanimoriginalrotation_yaw) (`KismetMathLibrary.BreakRotator` (`self.TempAnimOriginalRotation`)))
  ;[0.4342 0.1746 0] Drift Animation
  ;;[1 1 1] Deactivating Idle Anim
  (`self.StopIdleAnimTimeline`)
  (bind _output_get (set `self.TempAnimDriftRotation` (`KismetMathLibrary.RLerp` (`self.TempAnimOriginalRotation`) (select `bool` (`self.isDriftingToTheRight`) :`false` (`KismetMathLibrary.MakeRotator` -15.0 0.0 _tempanimoriginalrotation_yaw) :`true` (`KismetMathLibrary.MakeRotator` 15.0 0.0 _tempanimoriginalrotation_yaw)) (`self.TempLerpDrift`) true)))
  (`SceneComponent.K2_SetRelativeRotation` (`self.CarMesh`) _output_get false false))

(event `EndDriftAnimation`
  ;[0.4342 0.1746 0] End Drift Animation
  (bind (_direction _lerp) (`Timeline|EndDriftRotationAnimationLerp` :!via `PlayFromStart`)
    (:`Update`
      (`SceneComponent.K2_SetRelativeRotation` (`self.CarMesh`) (`KismetMathLibrary.RLerp` (`self.TempAnimDriftRotation`) (`self.TempAnimOriginalRotation`) _lerp true) false false))
    (:`Finished`
      ;;[1 1 1] If no other drift is initated, start Idle Animation
      (if (not (`self.isIdle`))
        (`self.CarIdleAnimation`)))))

(event `Impact Animation`
  (params (`Impact Normal` :type "Vector Structure"))
  (bind _returnvalue (`self.GetActorForwardVector`))
  (bind _returnvalue_2 (`self.GetActorRightVector`))
  ;[0.4342 0.1746 0] Impact Animation
  (if (> (`self.Speed`) 10.0)
    ;;[1 1 1] Deactivating Idle Anim
    (`self.StopIdleAnimTimeline`)
    (bind (_direction _lerpvalue0_6s) (`Timeline|ImpactAnimationLerp` :!via `PlayFromStart`)
      (:`Update`
        (`SceneComponent.K2_SetRelativeRotation` (`self.CarMesh`) (`KismetMathLibrary.RLerp` (`self.TempAnimOriginalRotation`) (select `int` (`KismetMathLibrary.MinOfFloatArray` (`|MakeArray` (`KismetMathLibrary.Dot_VectorVector` _returnvalue `Impact Normal`) (`KismetMathLibrary.Dot_VectorVector` `Impact Normal` (* _returnvalue -1.0)) (`KismetMathLibrary.Dot_VectorVector` _returnvalue_2 `Impact Normal`) (`KismetMathLibrary.Dot_VectorVector` `Impact Normal` (* _returnvalue_2 -1.0)))) :`0` (struct :`Pitch` 30.0 :`Yaw` 180.0) :`1` (struct :`Pitch` -30.0 :`Yaw` 180.0) :`2` (struct :`Yaw` 180.0 :`Roll` 30.0) :`3` (struct :`Yaw` 180.0 :`Roll` -30.0) :!type "Rotator Structure") _lerpvalue0_6s true) false false))
      (:`Finished`
        ;;[1 1 1] Reactivating Idle Animation
        (`self.CarIdleAnimation`)))))

(fn `ApplyGravity`
  (locals (FramesTheCarTakesToHitTheGround :type "Float (double-precision)" :default -30.0))
  (bind _returnvalue (`self.K2_GetActorLocation`))
  (bind _distancetoground (`self.DistanceToGround`))
  ;[1 1 1] Linetraces the floor towards the front of the vehicle
  (bind (_outhit _returnvalue_2) (`KismetSystemLibrary.BoxTraceSingle` _returnvalue (- _returnvalue (* (`self.GetActorUpVector`) 1000.0)) (100.0 100.0 1.0) (`self.K2_GetActorRotation`) "TraceTypeQuery1"))
  (if _returnvalue_2
    (bind (_returnvalue_x _returnvalue_y _returnvalue_z) (`KismetMathLibrary.BreakVector` (- (`.Location` (`GameplayStatics.BreakHitResult` _outhit)) (`self.K2_GetActorLocation`))))
    (bind _returnvalue_3 (`KismetMathLibrary.Sqrt` (`KismetMathLibrary.Square` _returnvalue_z)))
    ;[1 1 1] Check if the car is above or below the height it should be at
    (if (not (`KismetMathLibrary.NearlyEqual_FloatFloat` _returnvalue_3 _distancetoground 1.0))
      (bind _returnvalue_4 (- _returnvalue_3 _distancetoground))
      (if (< _returnvalue_4 0.0)
        (bind _returnvalue_5 (`KismetMathLibrary.Sqrt` (`KismetMathLibrary.Square` _returnvalue_4)))
        ;[1 1 1] If distance to floor is < DistanceToGround, add Z offset equal to that distance
        (`self.K2_AddActorWorldOffset` (`KismetMathLibrary.MakeVector` 0.0 0.0 _returnvalue_5) true)
        (else
          ;[1 1 1] If distance to floor is > DistanceToGround, add Z offset equal to that distance/Frames
          (`self.K2_AddActorWorldOffset` (`KismetMathLibrary.MakeVector` 0.0 0.0 (/ _returnvalue_5 (`local.FramesTheCarTakesToHitTheGround`))) true))))
    (else
      ;[1 1 1] If no floor detected, apply some gravity
      (`self.K2_AddActorWorldOffset` (0.0 0.0 -15.0) true))))

(fn `UserConstructionScript`)