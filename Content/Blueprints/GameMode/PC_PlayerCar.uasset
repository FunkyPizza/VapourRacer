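; Player controller for the hover car race that tracks one player's laps and finish time.
; BeginPlay caches the freestyle racing game mode and the possessed hover car.
; PlayerLap derives each lap time by subtracting the summed previous laps from the game mode's clock, then increments the lap counter.
; On the final lap it records the total time, notifies the game mode and stops the car.
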(event `self.ReceiveBeginPlay`
  ;[0.2344 0 0] Begin Play, Tick & Live Functions
  ;;[1 1 1] Setting default references
  (bind _asgm_freestyle_racing (cast `/Game/Blueprints/GameMode/GM_FreestyleRacing` (`GameplayStatics.GetGameMode`)))
  (set `self.GameMode` _asgm_freestyle_racing)
  (bind _returnvalue (`GameplayStatics.GetPlayerControllerID` self))
  (bind _asbp_hover_car (cast `/Game/Blueprints/Cars/BP_HoverCar` (`GameplayStatics.GetPlayerPawn` _returnvalue)))
  (set `self.Car` _asbp_hover_car))

(event `PlayerLap`
  ;[0 0 0] Adding lap to player & Checking if finished race
  ;;[1 1 1] Saving current lap time & recalculating total sum of lap times
  (`self.CalculateSumOfPreviousLaps`
    (:`Completed`
      (`KismetArrayLibrary.Array_Add` (`self.LapTimes`) (- (`/Game/Blueprints/GameMode/GM_FreestyleRacing.TimeValue` (`self.GameMode`)) (`self.TempSumOfPreviousLaps`)))
      (`self.CalculateSumOfPreviousLaps`
        (:`Completed`
          ;;[1 1 1] Adding lap to lap counter & checking if is final lap
          (`/Engine/EditorBlueprintResources/StandardMacros.IncrementInt` (`self.CurrentLap`)
            (:`  `
              (if (>= (`self.CurrentLap`) (`/Game/Blueprints/GameMode/GM_FreestyleRacing.MaxLap` (`self.GameMode`)))
                ;;[1 1 1] If it is the final lap, call game mode and stop player's movements
                (set `self.FinishTime` (`self.TempSumOfPreviousLaps`))
                (`/Game/Blueprints/GameMode/GM_FreestyleRacing.PlayerFinish` (`self.GameMode`) self)
                (`/Game/Blueprints/Cars/BP_HoverCar.StopMovements` (`self.Car`))))))))))

(fn `UserConstructionScript`)