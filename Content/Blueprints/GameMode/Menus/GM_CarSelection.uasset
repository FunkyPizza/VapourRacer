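; Game mode for the car selection menu, handling local multiplayer setup and ready-up before the race loads.
; On BeginPlay it has GI_VaporRacer spawn splitscreen players, then after a short delay sizes the ready array and shows each BP_CarSelector's UI.
; ReadyCheck and UnReadyPlayer track readiness; once all are ready, it clears controllers and opens the Loading level.
; ChoosePlayerStart matches PlayerStart tags to the last digit of the controller's name.
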(event `self.ReceiveBeginPlay`
  (bind _connectedplayercontrollers (`/Game/Blueprints/GameMode/GI_VaporRacer.ConnectedPlayerControllers` (`self.GameInstance`)))
  ;[0.2346 0 0] Begin Play & Tick
  (bind _asgi_vapor_racer (cast `/Game/Blueprints/GameMode/GI_VaporRacer` (`GameplayStatics.GetGameInstance`)))
  (set `self.GameInstance` _asgi_vapor_racer)
  ;;[1 1 1] Activate splitscreen if needed
  (`/Game/Blueprints/GameMode/GI_VaporRacer.SpawnAdditionalPlayers` (`self.GameInstance`))
  (`KismetSystemLibrary.Delay` 0.2)
  ;;[1 1 1] Make sure the PlayerReady array is the correct size
  (`KismetArrayLibrary.Array_Resize` (`self.PlayerReady`) (`KismetArrayLibrary.Array_Length` _connectedplayercontrollers))
  ;;[1 1 1] Once player have spawned, create their UI.
  (for _array_element _connectedplayercontrollers
    (bind _asbp_car_selector (cast `/Game/Blueprints/BP_CarSelector` (`Controller.K2_GetPawn` _array_element)))
    (`/Game/Blueprints/BP_CarSelector.DisplayUI` _asbp_car_selector)))

(event `ReadyCheck`
  (params (`ReadyPlayer'sID` :type Integer))
  ;[0 0 0] Check ready player & Load new map
  ;;[1 1 1] Set player ready
  (`KismetArrayLibrary.Array_Set` (`self.PlayerReady`) `ReadyPlayer'sID` true)
  ;;[1 1 1] Check if player is alone
  (if (== (`KismetArrayLibrary.Array_Length` (`self.PlayerReady`)) 1)
    (`/Game/Blueprints/GameMode/GI_VaporRacer.ClearPlayerControllers` (`self.GameInstance`) :!label _label)
    (`KismetSystemLibrary.Delay` 1.0)
    (`GameplayStatics.OpenLevel` "Loading")
    (else
      ;;[1 1 1] Check if all players are ready
      (`|ExecutionSequence`
        (:`then_0`
          (for _array_element (`self.PlayerReady`)
            (if (not _array_element)
              (set `self.bAllPlayersReady` false)))
          (if (`self.bAllPlayersReady`)
            (goto _label)))
        (:`then_1`
          (set `self.bAllPlayersReady` true))))))

(event `UnReady Player`
  (params (`ReadyPlayer'sID` :type Integer))
  ;[0 0 0] Check ready player & Load new map
  (`KismetArrayLibrary.Array_Set` (`self.PlayerReady`) `ReadyPlayer'sID`))

(fn `ChoosePlayerStart`
  (params (Player :type "Controller Object Reference"))
  (returns (ReturnValue :type "Actor Object Reference"))
  (locals (SelectedPlayerStart :type "PlayerStart Object Reference"))
  (bind _returnvalue (`KismetSystemLibrary.GetDisplayName` Player))
  (bind _outactors (`GameplayStatics.GetAllActorsOfClass` "/Script/Engine.PlayerStart"))
  (for _array_element _outactors
    (if (== (`KismetStringLibrary.Conv_StringToInt` (`KismetStringLibrary.Conv_NameToString` (`PlayerStart.PlayerStartTag` _array_element))) (`KismetStringLibrary.Conv_StringToInt` (`KismetStringLibrary.GetSubstring` _returnvalue (- (`KismetStringLibrary.Len` _returnvalue) 1))))
      (set `local.SelectedPlayerStart` _array_element)))
  (return (`local.SelectedPlayerStart`)))

(fn `UserConstructionScript`)