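; Game instance for VaporRacer that caps the frame rate at 60 on init and manages local multiplayer players.
; SpawnAdditionalPlayers sizes the controller and car arrays to AmountOfPlayers, stores player 0's controller, then creates the remaining players with pawns.
; GoBackToMainMenu removes every player except the first along with their pawns, waits briefly, then opens the MainMenu level.
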(event `self.ReceiveInit`
  (`KismetSystemLibrary.ExecuteConsoleCommand` "t.MaxFPS 60" null))

(event `SpawnAdditionalPlayers`
  ;[0 0 0] SpawnPlayers
  ;;[1 1 1] Set player array to No of Players
  (`KismetArrayLibrary.Array_Resize` (`self.ConnectedPlayerControllers`) (`self.AmountOfPlayers`))
  (`KismetArrayLibrary.Array_Resize` (`self.PlayerCars`) (`self.AmountOfPlayers`))
  ;;[1 1 1] Add Player 0 to array
  (`KismetArrayLibrary.Array_Set` (`self.ConnectedPlayerControllers`) 0 (`GameplayStatics.GetPlayerController` 0))
  ;;[1 1 1] Spawn additional players if needed
  (for _index (range 2 (+ (`self.AmountOfPlayers`) 1))
    (bind _returnvalue (- _index 1))
    (bind _returnvalue_2 (`GameplayStatics.CreatePlayer` _returnvalue))
    (`KismetArrayLibrary.Array_Set` (`self.ConnectedPlayerControllers`) _returnvalue _returnvalue_2)))

(event `GoBackToMainMenu`
  ;[0 0 0] SpawnPlayers
  ;;[1 1 1] Remove players and go back to main menu
  (`self.ClearPlayerControllers`)
  (`KismetSystemLibrary.Delay` 0.5)
  (`GameplayStatics.OpenLevel` "MainMenu"))

(event `ClearPlayerControllers`
  ;[0 0 0] SpawnPlayers
  (for (_array_element _array_index) (`self.ConnectedPlayerControllers`)
    (if (!= _array_index 0)
      (`GameplayStatics.RemovePlayer` _array_element true))))