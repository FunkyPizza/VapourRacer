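; Game mode for local multiplayer freestyle hover car racing in VaporRacer.
; BeginPlay spawns extra players through the game instance, adds per-player UI, waits, then enables car movement and counts elapsed time on Tick.
; Pawn class and tagged start follow the last digit of each controller's display name.
; The win widget names the first finisher once all finish; the countdown leading to draw and level reload is never called.
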(event `self.ReceiveBeginPlay`
  ;[0.2344 0 0] Begin Play, Tick & Live Functions
  ;;[1 1 1] Setting variables from game instance
  (bind _asgi_vapor_racer (cast `/Game/Blueprints/GameMode/GI_VaporRacer` (`GameplayStatics.GetGameInstance`)))
  (bind _output_get (set `self.GameInstance` _asgi_vapor_racer))
  (set `self.AmountOfPlayers` (`/Game/Blueprints/GameMode/GI_VaporRacer.AmountOfPlayers` _output_get))
  (`/Game/Blueprints/GameMode/GI_VaporRacer.SpawnAdditionalPlayers` _output_get)
  (set `self.PlayerControllers` (`/Game/Blueprints/GameMode/GI_VaporRacer.ConnectedPlayerControllers` _output_get))
  (`KismetSystemLibrary.Delay` 0.2)
  (`self.DisplayPlayerUIs`)
  (`KismetSystemLibrary.Delay` 2.0)
  ;;[1 1 1] Temporary countdown
  (`KismetSystemLibrary.Delay` 3.0)
  (`KismetSystemLibrary.PrintString` "GO " true true (struct :`R` 0.236033 :`G` 1.0 :`A` 1.0))
  ;;[1 1 1] Starting the race
  (`self.SetTimer` (`self.DefaultTimerValue`))
  (`self.StartTimer`)
  (`self.ReadyPlayers`))

(event `self.ReceiveTick`
  (params (DeltaSeconds :type "Float (single-precision)"))
  ;[0.2344 0 0] Begin Play, Tick & Live Functions
  (`self.Time`))

(event `PlayerFinish`
  (params (`Winning Player` :type "/Game/Blueprints/GameMode/PC_PlayerCar Object Reference"))
  ;[0 0 0] Victory & Lose Conditions
  ;;[1 1 1] Player finish
  (`KismetArrayLibrary.Array_Add` (`self.FinishedPlayers`) `Winning Player`)
  (if (== (`KismetArrayLibrary.Array_Length` (`self.FinishedPlayers`)) (`KismetArrayLibrary.Array_Length` (`self.PlayerControllers`)))
    (bind _returnvalue (`GameplayStatics.GetPlayerControllerID` (`|GetArrayItem` (`self.FinishedPlayers`))))
    (bind _returnvalue_2 (`|CreateWidget` "/Game/Blueprints/UserInterface/InGame/W_Win.W_Win_C" null _returnvalue))
    (`UserWidget.AddToViewport` _returnvalue_2 0)))

(event `StartTimer`
  ;[0 0 0] Timer Control
  ;;[1 1 1] Controls
  (set `self.isTimedStopped` true))

(event `StopTimer`
  ;[0 0 0] Timer Control
  ;;[1 1 1] Controls
  (set `self.isTimedStopped` false))

(event `SetTimer`
  (params (`Timer Value` :type "Float (double-precision)"))
  ;[0 0 0] Timer Control
  ;;[1 1 1] Controls
  (set `self.TimerValue` `Timer Value`))

(event `Time`
  ;[0 0 0] Timer Control
  ;;[1 1 1] Time
  (if (`self.isTimedStopped`)
    (set `self.TimeValue` (+ (`self.TimeValue`) (`GameplayStatics.GetWorldDeltaSeconds`)))))

(event `PlayerLoose`
  ;[0 0 0] Victory & Lose Conditions
  ;;[1 1 1] Player loose
)

(event `Timer`
  ;[0 0 0] Timer Control
  ;;[1 1 1] Timer
  (bind _output_get (set `self.TimerValue` (`KismetMathLibrary.FClamp` (- (`self.TimerValue`) (`GameplayStatics.GetWorldDeltaSeconds`)) -0.1 1000.0)))
  (if (<= _output_get 0.0)
    (`self.TimerRanOut`)))

(event `TimerRanOut`
  ;[0 0 0] Victory & Lose Conditions
  ;;[1 1 1] Timer ran out
  (`/Engine/EditorBlueprintResources/StandardMacros.DoOnce` false
    (:`Completed`
      (bind _returnvalue (`|CreateWidget` "/Game/Blueprints/UserInterface/InGame/W_Draw.W_Draw_C"))
      (`UserWidget.AddToViewport` _returnvalue 0)
      (`KismetSystemLibrary.Delay` 3.0)
      (bind _returnvalue_2 (`GameplayStatics.GetCurrentLevelName` true))
      (`GameplayStatics.OpenLevel` (`KismetStringLibrary.Conv_StringToName` _returnvalue_2)))))

(event `ReadyPlayers`
  ;[0 0 0] Player Setup
  (for _array_element (`/Game/Blueprints/GameMode/GI_VaporRacer.ConnectedPlayerControllers` (`self.GameInstance`))
    (bind _returnvalue (`GameplayStatics.GetPlayerControllerID` _array_element))
    (bind _asbp_hover_car (cast `/Game/Blueprints/Cars/BP_HoverCar` (`GameplayStatics.GetPlayerPawn` _returnvalue)))
    (`/Game/Blueprints/Cars/BP_HoverCar.StartMovements` _asbp_hover_car)))

(event `DisplayPlayerUIs`
  ;[0 0 0] Player Setup
  (for _array_element (`/Game/Blueprints/GameMode/GI_VaporRacer.ConnectedPlayerControllers` (`self.GameInstance`))
    (bind _returnvalue (`GameplayStatics.GetPlayerControllerID` _array_element))
    (bind _asbp_hover_car (cast `/Game/Blueprints/Cars/BP_HoverCar` (`GameplayStatics.GetPlayerPawn` _returnvalue)))
    (bind _returnvalue_2 (`|CreateWidget` "/Game/Blueprints/UserInterface/InGame/W_UI.W_UI_C" _array_element))
    (bind _output_get (set `/Game/Blueprints/Cars/BP_HoverCar.UIWidget` _returnvalue_2 _asbp_hover_car))
    (`UserWidget.AddToPlayerScreen` _output_get 0)))

(fn `ChoosePlayerStart`
  (params (Player :type "Controller Object Reference"))
  (returns (ReturnValue :type "Actor Object Reference"))
  (locals (SelectedPlayerStart :type "PlayerStart Object Reference"))
  (bind _returnvalue (`KismetSystemLibrary.GetDisplayName` Player))
  (bind _outactors (`GameplayStatics.GetAllActorsOfClass` "/Script/Engine.PlayerStart"))
  (for _array_element _outactors
    (if (== (`KismetStringLibrary.Conv_StringToInt` (`KismetStringLibrary.Conv_NameToString` (`PlayerStart.PlayerStartTag` _array_element))) (`KismetStringLibrary.Conv_StringToInt` (`KismetStringLibrary.GetSubstring` _returnvalue (- (`KismetStringLibrary.Len` _returnvalue) 1))))
      (set `local.SelectedPlayerStart` _array_element)))
  (return (`local.SelectedPlayerStart`)))

(fn `GetDefaultPawnClassForController`
  (params (InController :type "Controller Object Reference"))
  (returns (ReturnValue :type "Object Class Reference"))
  (bind _returnvalue (`KismetSystemLibrary.GetDisplayName` InController))
  (bind _asgi_vapor_racer (cast `/Game/Blueprints/GameMode/GI_VaporRacer` (`GameplayStatics.GetGameInstance`) :!pure true))
  (bind _returnvalue_2 (`KismetStringLibrary.Conv_StringToInt` (`KismetStringLibrary.GetSubstring` _returnvalue (- (`KismetStringLibrary.Len` _returnvalue) 1))))
  (`KismetSystemLibrary.PrintString` (`KismetStringLibrary.Conv_IntToString` _returnvalue_2))
  (return (`|GetArrayItem` (`/Game/Blueprints/GameMode/GI_VaporRacer.CarList` _asgi_vapor_racer) (`|GetArrayItem` (`/Game/Blueprints/GameMode/GI_VaporRacer.PlayerCars` _asgi_vapor_racer) _returnvalue_2))))

(fn `UserConstructionScript`)