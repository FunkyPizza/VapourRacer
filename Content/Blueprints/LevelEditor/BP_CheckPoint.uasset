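; BP_CheckPoint is a lap checkpoint for the hover car racing game, triggered when a BP_HoverCar overlaps its box.
; It compares the sweep normal with the arrow's forward vector to accept only one crossing direction.
; A valid crossing calls PlayerLap on the car's PC_PlayerCar and adds a lap time to its UI widget.
; A LastPlayerCollided guard targets repeat triggers, but is cleared right after each counted lap.
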(event `self.ReceiveBeginPlay`
  ;[0.2344 0 0] Begin Play, Tick & Live Functions
  ;;[1 1 1] Setting default references
  (bind _asgm_freestyle_racing (cast `/Game/Blueprints/GameMode/GM_FreestyleRacing` (`GameplayStatics.GetGameMode`)))
  (set `self.GameMode` _asgm_freestyle_racing))

(event `self.Box.OnComponentBeginOverlap`
  (params (OverlappedComponent :type "PrimitiveComponent Object Reference") (OtherActor :type "Actor Object Reference") (OtherComp :type "PrimitiveComponent Object Reference") (OtherBodyIndex :type Integer) (bFromSweep :type Boolean) (SweepResult :type "HitResult Structure (by ref)"))
  ;[0 0 0] Collision with player
  (bind _asbp_hover_car (cast `/Game/Blueprints/Cars/BP_HoverCar` OtherActor))
  (if (> (`KismetMathLibrary.Dot_VectorVector` SweepResult_Normal (`KismetMathLibrary.Conv_RotatorToVector` (`SceneComponent.K2_GetComponentRotation` (`self.Arrow`)))) 0.0)
    ;;[1 1 1] Making sure that it will trigger only once per lap
    (if (!= (`self.LastPlayerCollided`) _asbp_hover_car)
      (set `self.LastPlayerCollided` _asbp_hover_car)
      ;;[1 1 1] If player collided in the correct way call its player controller
      (bind _asplayer_controller (cast `PlayerController` (`Pawn.GetController` _asbp_hover_car)))
      (bind _aspc_player_car (cast `/Game/Blueprints/GameMode/PC_PlayerCar` _asplayer_controller))
      (`/Game/Blueprints/GameMode/PC_PlayerCar.PlayerLap` _aspc_player_car)
      (`/Game/Blueprints/UserInterface/InGame/W_UI.AddLapTime` (`/Game/Blueprints/Cars/BP_HoverCar.UIWidget` _asbp_hover_car))
      (set `self.LastPlayerCollided` null)
      (elif (== (`/Game/Blueprints/GameMode/GM_FreestyleRacing.AmountOfPlayers` (`self.GameMode`)) 1)
        (set `self.LastPlayerCollided` null)))))

(fn `UserConstructionScript`)