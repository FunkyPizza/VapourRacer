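; Per-player car selection actor for VaporRacer that shows a spinning preview car and the W_CarSelect widget.
; MoveRight input, gated by a DoOnce cooldown, steps through the game instance's CarList, spawning each car to one side while timelines slide it in and the old one out before destroying it.
; Bottom face button toggles ready, saving the choice to PlayerCars and notifying GM_CarSelection; right face button returns to the main menu.
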(event `self.ReceiveBeginPlay`
  ;[0.2346 0 0] Begin Play & Tick
  (set `self.GameInstance` (cast `/Game/Blueprints/GameMode/GI_VaporRacer` (`GameplayStatics.GetGameInstance`) :!pure true)))

(event `DisplayUI`
  ;[0.2346 0 0] Begin Play & Tick
  (bind _asplayer_controller (cast `PlayerController` (`self.GetController`)))
  (`WidgetBlueprintLibrary.SetInputMode_GameOnly` _asplayer_controller)
  (`self.SpawnNextCar`)
  (bind _returnvalue (`|CreateWidget` "/Game/Blueprints/UserInterface/Menus/W_CarSelect.W_CarSelect_C" _asplayer_controller))
  (`UserWidget.AddToPlayerScreen` _returnvalue 0))

(event `self.ReceiveTick`
  (params (DeltaSeconds :type "Float (single-precision)"))
  (bind _currentcar (`self.CurrentCar`))
  ;[0.2346 0 0] Begin Play & Tick
  (`/Engine/EditorBlueprintResources/StandardMacros.IsValid` _currentcar
    (:`Is Valid`
      (`SceneComponent.K2_AddLocalRotation` (`Actor.RootComponent` _currentcar) (struct :`Yaw` 0.1) false false))))

(event `InputAxis|MoveRight`
  (params (AxisValue :type "Float (single-precision)"))
  (bind _returnvalue (>= AxisValue 0.5))
  (bind _returnvalue_2 (<= AxisValue -0.5))
  ;[0 0 0] Player input
  ;;[1 1 1] Select Left/Right
  (if (or _returnvalue _returnvalue_2)
    (`/Engine/EditorBlueprintResources/StandardMacros.DoOnce` false :!label _label
      (:`Completed`
        ;;;[1 1 1] Right
        (if _returnvalue_2
          (`self.SpawnPreviousCar`)
          (`KismetSystemLibrary.RetriggerableDelay` 1.0 :!label _label_2)
          (`self.CarSwapCoolDownReset`)
          (else
            ;;;[1 1 1] Left
            (if _returnvalue
              (`self.SpawnNextCar`)
              (goto _label_2))))))))

(event `Key|Gamepad_FaceButton_Right`
  (params (Key :type "Key Structure"))
  ;[0 0 0] Player input
  ;;[1 1 1] Accept selection
  (:`Pressed`
    (`/Game/Blueprints/GameMode/GI_VaporRacer.GoBackToMainMenu` (`self.GameInstance`))))

(event `CarSwapCoolDownReset`
  ;[0 0 0] Player input
  ;;[1 1 1] Select Left/Right
  (goto _label :!via `Reset`))

(event `Key|Gamepad_FaceButton_Bottom`
  (params (Key :type "Key Structure"))
  ;[0 0 0] Player input
  ;;[1 1 1] Accept selection
  (:`Pressed`
    (`/Engine/EditorBlueprintResources/StandardMacros.FlipFlop`
      (:`A`
        (bind _returnvalue (`GameplayStatics.GetPlayerControllerID` (cast `PlayerController` (`self.GetController`) :!pure true)))
        (`KismetArrayLibrary.Array_Set` (`/Game/Blueprints/GameMode/GI_VaporRacer.PlayerCars` (`self.GameInstance`)) _returnvalue (`self.SelectedCar`))
        (`/Game/Blueprints/GameMode/Menus/GM_CarSelection.ReadyCheck` (cast `/Game/Blueprints/GameMode/Menus/GM_CarSelection` (`GameplayStatics.GetGameMode`) :!pure true) _returnvalue)
        (set `self.isReady` true))
      (:`B`
        (bind _returnvalue_2 (`GameplayStatics.GetPlayerControllerID` (cast `PlayerController` (`self.GetController`) :!pure true)))
        (`/Game/Blueprints/GameMode/Menus/GM_CarSelection.UnReady Player` (cast `/Game/Blueprints/GameMode/Menus/GM_CarSelection` (`GameplayStatics.GetGameMode`) :!pure true) _returnvalue_2)
        (set `self.isReady` false)))))

(event `SpawnNextCar`
  (bind _currentcar (`self.CurrentCar`))
  (bind _returnvalue (+ (`self.SelectedCar`) 1))
  (bind _returnvalue_2 (`KismetArrayLibrary.Array_LastIndex` (`/Game/Blueprints/GameMode/GI_VaporRacer.CarList` (`self.GameInstance`))))
  ;[0 0 0] Car Spawning
  ;;[1 1 1] Get car class from GI Car Array
  (if (> _returnvalue _returnvalue_2)
    (`self.CarSwapCoolDownReset`)
    (else
      (set `self.SelectedCar` (`KismetMathLibrary.Clamp` _returnvalue 0 _returnvalue_2))
      ;;[1 1 1] Remove Current Car
      (`/Engine/EditorBlueprintResources/StandardMacros.IsValid` _currentcar
        (:`Is Valid`
          (bind _output_get (set `self.LastSpawnedCar` _currentcar))
          (`self.MoveAndDestroyCar` _output_get true))
        (:`Is Not Valid`
          _))
      ;;[1 1 1] Spawn the car
      (bind _returnvalue_3 (`|SpawnActorFromClass` (`|GetArrayItem` (`/Game/Blueprints/GameMode/GI_VaporRacer.CarList` (`self.GameInstance`)) (`self.SelectedCar`)) (`KismetMathLibrary.MakeTransform` (+ (`self.K2_GetActorLocation`) (`self.GetRightRelativeTargetLocation`)) (struct :`Yaw` 180.0)) "AlwaysSpawn" "OverrideRootScale" null null))
      (bind _output_get_2 (set `self.CurrentCar` _returnvalue_3))
      ;;[1 1 1] New car appear animation
      (`self.MoveCar` _output_get_2 true))))

(event `SpawnPreviousCar`
  (bind _currentcar (`self.CurrentCar`))
  (bind _returnvalue (- (`self.SelectedCar`) 1))
  ;[0 0 0] Car Spawning
  ;;[1 1 1] Get car class from GI Car Array
  (if (< _returnvalue 0)
    (`self.CarSwapCoolDownReset`)
    (else
      (set `self.SelectedCar` (`KismetMathLibrary.Clamp` _returnvalue 0 (`KismetArrayLibrary.Array_LastIndex` (`/Game/Blueprints/GameMode/GI_VaporRacer.CarList` (`self.GameInstance`)))))
      ;;[1 1 1] Remove Current Car
      (`/Engine/EditorBlueprintResources/StandardMacros.IsValid` _currentcar
        (:`Is Valid`
          (bind _output_get (set `self.LastSpawnedCar` _currentcar))
          (`self.MoveAndDestroyCar` _output_get))
        (:`Is Not Valid`
          _))
      ;;[1 1 1] Spawn the car
      (bind _returnvalue_2 (`|SpawnActorFromClass` (`|GetArrayItem` (`/Game/Blueprints/GameMode/GI_VaporRacer.CarList` (`self.GameInstance`)) (`self.SelectedCar`)) (`KismetMathLibrary.MakeTransform` (+ (`self.K2_GetActorLocation`) (`self.GetLeftRelativeTargetLocation`)) (struct :`Yaw` 180.0)) "AlwaysSpawn" "OverrideRootScale" null null))
      (bind _output_get_2 (set `self.CurrentCar` _returnvalue_2))
      ;;[1 1 1] New car appear animation
      (`self.MoveCar` _output_get_2))))

(event `MoveAndDestroyCar`
  (params (CarToDisappear :type "/Game/Blueprints/Cars/BP_HoverCar Object Reference") (isMovingLeft :type Boolean))
  (bind (_returnvalue_x _returnvalue_y _returnvalue_z) (`KismetMathLibrary.BreakVector` (`self.K2_GetActorLocation` CarToDisappear)))
  (bind _tempcarinitiallocation2 (`self.TempCarInitialLocation2`))
  ;[0.4342 0.1746 0] Car animation
  (set `self.TempCarInitialLocation2` (`self.K2_GetActorLocation` CarToDisappear))
  (bind (_direction _lerp) (`Timeline|CarAnim_Lerp1` :!via `PlayFromStart`)
    (:`Update`
      (bind (_returnvalue_x_2 _returnvalue_y_2) (`KismetMathLibrary.BreakVector` (`KismetMathLibrary.VLerp` _tempcarinitiallocation2 (+ _tempcarinitiallocation2 (select `bool` isMovingLeft :`false` (`self.GetRightRelativeTargetLocation`) :`true` (`self.GetLeftRelativeTargetLocation`))) _lerp)))
      (`self.K2_SetActorLocation` CarToDisappear (`KismetMathLibrary.MakeVector` _returnvalue_x_2 _returnvalue_y_2 _returnvalue_z) false false))
    (:`Finished`
      (`self.K2_DestroyActor` CarToDisappear))))

(event `MoveCar`
  (params (CarToAppear :type "/Game/Blueprints/Cars/BP_HoverCar Object Reference") (isMovingLeft :type Boolean))
  (bind (_returnvalue_x _returnvalue_y _returnvalue_z) (`KismetMathLibrary.BreakVector` (`self.K2_GetActorLocation` CarToAppear)))
  (bind _tempcarinitallocation1 (`self.TempCarInitalLocation1`))
  ;[0.4342 0.1746 0] Car animation
  (set `self.TempCarInitalLocation1` (`self.K2_GetActorLocation` CarToAppear))
  (bind (_direction _lerp) (`Timeline|Timeline_0` :!via `PlayFromStart`)
    (:`Update`
      (bind (_returnvalue_x_2 _returnvalue_y_2) (`KismetMathLibrary.BreakVector` (`KismetMathLibrary.VLerp` _tempcarinitallocation1 (+ _tempcarinitallocation1 (select `bool` isMovingLeft :`false` (`self.GetRightRelativeTargetLocation`) :`true` (`self.GetLeftRelativeTargetLocation`))) _lerp)))
      (`self.K2_SetActorLocation` CarToAppear (`KismetMathLibrary.MakeVector` _returnvalue_x_2 _returnvalue_y_2 _returnvalue_z) false false))))

(fn `SetCarLocationRelativeToActorNoZ`
  (params (TargetLocation :type "Vector Structure") (Lerp :type "Float (double-precision)") (Car :type "/Game/Blueprints/Cars/BP_HoverCar Object Reference"))
  (bind (_returnvalue_x _returnvalue_y _returnvalue_z) (`KismetMathLibrary.BreakVector` (`self.K2_GetActorLocation` Car)))
  (bind _tempcarinitiallocation2 (`self.TempCarInitialLocation2`))
  (bind (_returnvalue_x_2 _returnvalue_y_2) (`KismetMathLibrary.BreakVector` (`KismetMathLibrary.VLerp` _tempcarinitiallocation2 (+ _tempcarinitiallocation2 TargetLocation) Lerp)))
  (`self.K2_SetActorLocation` Car (`KismetMathLibrary.MakeVector` _returnvalue_x_2 _returnvalue_y_2 _returnvalue_z) false false))

(fn `UserConstructionScript`)